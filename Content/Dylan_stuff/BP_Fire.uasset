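; BP_Fire is a fire hazard actor that knocks the third-person player character back on overlap and can be removed through interaction.
; On overlap, it launches the character along the negated capsule forward vector, converted into the fire actor's local space and scaled to a fixed strength.
; The InteractionInterface event destroys the actor, and the PlayerName function returns an empty string.
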(event Collision|EventActorBeginOverlap
  (params (OtherActor :type Actor%20Object%20Reference))
  (bind _asbp_third_person_character (Utilities|Casting|CastToBP_ThirdPersonCharacter OtherActor))
  (Character|LaunchCharacter _asbp_third_person_character (* (Math|Transform|InverseTransformDirection (Transformation|GetActorTransform) (Math|Vector|GetForwardVector (Variables|/Script/Engine.Character|GetCapsuleComponent _asbp_third_person_character))) -1.5e+03) false false))

(event EventInteractionInterface
  (params (Actor%20who%20interacted :type Actor%20Object%20Reference))
  (Actor|DestroyActor))

(fn ConstructionScript)

(fn PlayerName
  (return ""))